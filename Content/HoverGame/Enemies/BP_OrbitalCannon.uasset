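; Orbital cannon enemy that, while bombing is active, targets BP_OrbitalExplosion strikes at the player hovercraft's predicted position.
; Each tick it extrapolates the craft's MovementDirection 1.3 seconds ahead and traces vertically against WorldStatic for the impact point.
; A live explosion has its TargetLocation updated to that point, so it keeps tracking the prediction.
; Otherwise a new one spawns there, gated by a DoOnce that resets after a six-second delay.
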(event `self.ReceiveTick`
  (params (DeltaSeconds :type "Float (single-precision)"))
  (bind (_prediction _success) (`self.PredictPlayerLocation` 1.3))
  (bind _currentexplosion (`self.CurrentExplosion`))
  (if (`self.BombingActive`)
    (set `self.Prediction` _prediction)
    (if _success
      (bind _outhit (`KismetSystemLibrary.LineTraceSingleForObjects` (+ (`self.Prediction`) (0.0 0.0 100000.0)) (+ (`self.Prediction`) (0.0 0.0 -100000.0)) (`|MakeArray` "ObjectTypeQuery1" :!type "EObjectTypeQuery Enum")))
      (`/Engine/EditorBlueprintResources/StandardMacros.IsValid` _currentexplosion
        (:`Is Valid`
          (bind (_bblockinghit _binitialoverlap _time _distance _location) (`GameplayStatics.BreakHitResult` _outhit))
          (set `/Game/HoverGame/Enemies/BP_OrbitalExplosion.TargetLocation` _location _currentexplosion))
        (:`Is Not Valid`
          (`/Engine/EditorBlueprintResources/StandardMacros.DoOnce` false :!label _label
            (:`Completed`
              (bind _returnvalue (`|SpawnActorFromClass` "/Game/HoverGame/Enemies/BP_OrbitalExplosion.BP_OrbitalExplosion_C" (`KismetMathLibrary.MakeTransform` _location) "Undefined" "OverrideRootScale" null (`self.GetInstigator`)))
              (set `self.CurrentExplosion` _returnvalue)
              (`KismetSystemLibrary.Delay` 6.0)
              (goto _label :!via `Reset`))))))))

(fn `PredictPlayerLocation`
  (params (Time :type "Float (double-precision)"))
  (returns (Prediction :type "Vector Structure") (Success :type Boolean))
  (bind _asbp_player_hovercraft (cast `/Game/HoverGame/Player/BP_PlayerHovercraft` (`GameplayStatics.GetPlayerPawn` 0))
    (:`then`
      (return (+ (* (`/Game/HoverGame/Player/BP_PlayerHovercraft.MovementDirection` _asbp_player_hovercraft) Time) (`self.K2_GetActorLocation` _asbp_player_hovercraft)) true))
    (:`CastFailed`
      (return (0.0 0.0 0.0) false))))

(fn `UserConstructionScript`)