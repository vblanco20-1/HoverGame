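; Player hovercraft pawn with physics-based hovering, jumping, twin guns and lock-on missiles.
; Four line-traced thrusters push the box body up and set damping by ground contact, while torque turns it toward the view and an anti-flip force rights it.
; A camera trace aims both child-actor guns; holding Missile selects targets, releasing launches homing missiles.
; Also creates the game HUD, routes radial damage and respawns at the start location on death.
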(event `self.ReceiveTick`
  (params (DeltaSeconds :type "Float (single-precision)"))
  (bind _box (`self.Box`))
  ;[1 1 1] General Update
  (`|ExecutionSequence`
    (:`then_0`
      (`self.UpdateInput`)
      ;[1 0.5559 0.4961] Physics Update
      (`|ExecutionSequence`
        (:`then_0`
          ;;[1 1 1] Update Thrusters
          (if (`self.UseThrusters`)
            (set `self.Thruster Hits` 0)
            (`self.CalculateThruster` (`self.Thruster1`))
            (`self.CalculateThruster` (`self.Scene`))
            (`self.CalculateThruster` (`self.Scene1`))
            (`self.CalculateThruster` (`self.Scene2`))))
        (:`then_1`
          ;;[1 1 1] Dampen physics when touching floor
          (`/Engine/EditorBlueprintResources/StandardMacros.CompareInt` (`self.Thruster Hits`) 2
            (:`>`
              (`PrimitiveComponent.SetLinearDamping` _box 5.0 :!label _label)
              (set `self.nJumps` 0))
            (:`==`
              (goto _label))
            (:`<`
              (`PrimitiveComponent.SetLinearDamping` _box 1.0))))
        (:`then_2`
          ;;[1 1 1] Add force to align with view
          (`PrimitiveComponent.AddTorqueInRadians` (`self.Box`) (`KismetMathLibrary.MakeVector` 0.0 0.0 (* (.y (`KismetMathLibrary.TransformDirection` (`KismetMathLibrary.InvertTransform` (`SceneComponent.K2_GetComponentToWorld` (`self.Box`))) (`KismetMathLibrary.GetForwardVector` (`self.GetControlRotation`)))) 10000000.0)) "None" false))))
    (:`then_1`
      (`self.Aim`))
    (:`then_2`
      (`self.AntiFlip`))
    (:`then_3`
      (`self.UpdateTargetting` DeltaSeconds))
    (:`then_4`
      (set `self.MovementDirection` (/ (- (`self.K2_GetActorLocation`) (`self.LastLocation`)) DeltaSeconds))
      (set `self.LastLocation` (`self.K2_GetActorLocation`)))))

(event `InputAction|Jump`
  (params (Key :type "Key Structure"))
  (bind _njumps (`self.nJumps`))
  ;[1 1 1] Jump Logic
  (:`Pressed`
    (if (== _njumps 0)
      (`/Engine/EditorBlueprintResources/StandardMacros.IncrementInt` _njumps
        (:`  `
          (`PrimitiveComponent.AddImpulse` (`self.Box`) (0.0 0.0 400000.0) "None" false)
          (set `self.UseThrusters` false)
          (`KismetSystemLibrary.Delay` 0.3)
          (set `self.UseThrusters` true))))))

(event `InputAction|AltFire`
  (params (Key :type "Key Structure"))
  ;[1 0.2772 0.1573] Shotgun Fire
  (:`Pressed`
    (`/Engine/EditorBlueprintResources/StandardMacros.DoOnce` false :!label _label_2
      (:`Completed`
        (for _array_element (`self.GetGuns`)
          (`/Game/HoverGame/Weapons/BP_HovercraftGun.Shotgun` _array_element))
        (`|ExecutionSequence`
          (:`then_0`
            (`KismetSystemLibrary.Delay` 1.0)
            (goto _label_2 :!via `Reset`))
          (:`then_1`
            (`PlayerCameraManager.PlayCameraShake` :`self` (`GameplayStatics.GetPlayerCameraManager` 0) :`ShakeClass` "/Game/HoverGame/Player/ShootingShake.ShootingShake_C" :`Scale` 3.0)))))))

(event `InputAction|Fire`
  (params (Key :type "Key Structure"))
  (bind _newparam (`self.GetGuns`))
  ;[1 0.2772 0.1573] Fire input
  (:`Pressed`
    (for _array_element _newparam
      (set `/Game/HoverGame/Weapons/BP_HovercraftGun.Fire` true _array_element)))
  (:`Released`
    (for _array_element_2 _newparam
      (set `/Game/HoverGame/Weapons/BP_HovercraftGun.Fire` false _array_element_2))))

(event `self.ReceiveBeginPlay`
  ;[1 1 1] Initialization
  (`|ExecutionSequence`
    (:`then_0`
      (bind _returnvalue (`|CreateWidget` "/Game/HoverGame/UI/WBP_GameUI.WBP_GameUI_C" (`GameplayStatics.GetPlayerController` 0)))
      (`UserWidget.AddToViewport` _returnvalue 0))
    (:`then_1`
      (set `self.StartLocation` (`self.K2_GetActorLocation`)))))

(event `self.ReceiveRadialDamage`
  (params (DamageReceived :type "Float (single-precision)") (DamageType :type "DamageType Object Reference") (Origin :type "Vector Structure") (HitInfo :type "HitResult Structure (by ref)") (InstigatedBy :type "Controller Object Reference") (DamageCauser :type "Actor Object Reference"))
  ;[1 1 1] Route Radial Damage
  (`DamageComponent.ApplyDamage` (`self.Damage`) HitInfo "/Script/Engine.DamageType" DamageReceived InstigatedBy DamageCauser))

(event `InputAction|Missile`
  (params (Key :type "Key Structure"))
  (bind _selectedtargets (`TargetSelectionComponent.SelectedTargets` (`self.TargetSelection`)))
  ;[1 1 1] Launch missiles
  (:`Pressed`
    (set `self.SelectTargets` true))
  (:`Released`
    (set `self.SelectTargets` false)
    (for _array_element _selectedtargets
      (`self.LaunchMisileAt` (`ActorComponent.GetOwner` _array_element)))
    (`KismetArrayLibrary.Array_Clear` _selectedtargets)
    (bind _outactors (`GameplayStatics.GetAllActorsOfClass` "/Game/HoverGame/UI/BP_TargetReticle.BP_TargetReticle_C"))
    (for _array_element_2 _outactors
      (`self.K2_DestroyActor` _array_element_2))))

(event `self.Damage.OnDeath`
  (params (Event :type "HoverDeathEvent Structure"))
  ;[1 1 1] Death Logic: Respawn
  (`self.K2_SetActorLocation` (`self.StartLocation`))
  (`KismetSystemLibrary.Delay` 0.2)
  (`DamageComponent.Restore` (`self.Damage`)))

(fn `Aim`
  (bind _returnvalue (`GameplayStatics.GetPlayerCameraManager` 0))
  (bind _returnvalue_2 (`self.K2_GetActorLocation` _returnvalue))
  (bind _returnvalue_3 (+ (* (`self.GetActorForwardVector` _returnvalue) 10000.0) _returnvalue_2))
  (bind (_outhit _returnvalue_4) (`KismetSystemLibrary.LineTraceSingle` _returnvalue_2 _returnvalue_3 "TraceTypeQuery1"))
  (`|ExecutionSequence`
    (:`then_0`
      (bind _asbp_hovercraft_gun (cast `/Game/HoverGame/Weapons/BP_HovercraftGun` (`ChildActorComponent.ChildActor` (`self.ChildActor1`))))
      (bind (_bblockinghit _binitialoverlap _time _distance _location _impactpoint) (`GameplayStatics.BreakHitResult` _outhit))
      (bind _returnvalue_5 (+ (select `bool` (< _distance 1000.0) :`false` (`KismetMathLibrary.SelectVector` _impactpoint _returnvalue_3 _returnvalue_4) :`true` _returnvalue_3) (0.0 0.0 100.0)))
      (`/Game/HoverGame/Weapons/BP_HovercraftGun.SetTarget` _asbp_hovercraft_gun _returnvalue_5))
    (:`then_1`
      (bind _asbp_hovercraft_gun_2 (cast `/Game/HoverGame/Weapons/BP_HovercraftGun` (`ChildActorComponent.ChildActor` (`self.ChildActor`))))
      (`/Game/HoverGame/Weapons/BP_HovercraftGun.SetTarget` _asbp_hovercraft_gun_2 _returnvalue_5))))

(fn `AntiFlip`
  (bind _returnvalue (`SceneComponent.K2_GetComponentLocation` (`self.Box`)))
  (bind _returnvalue_2 (`SceneComponent.K2_GetComponentLocation` (`self.AntiflipSensor`)))
  (`KismetSystemLibrary.DrawDebugLine` _returnvalue_2 (+ _returnvalue (0.0 0.0 100.0)))
  (`PrimitiveComponent.AddForceAtLocation` (`self.Box`) (* (* (- _returnvalue _returnvalue_2) 1000.0) (1.0 1.0 0.0)) (`SceneComponent.K2_GetComponentLocation` (`self.AntiflipSensor`)) "None"))

(fn `CalculateThruster`
  (params (Thruster :type "SceneComponent Object Reference"))
  (returns (HitsFloor :type Boolean))
  (bind _returnvalue (`SceneComponent.K2_GetComponentLocation` Thruster))
  (bind _thruster (`local.Thruster`))
  (bind (_outhit _returnvalue_2) (`KismetSystemLibrary.LineTraceSingle` :`Start` _returnvalue :`End` (+ _returnvalue (* (`SceneComponent.GetUpVector` Thruster) -150.0)) :`TraceChannel` "TraceTypeQuery1" :`DrawDebugType` "ForOneFrame"))
  (if _returnvalue_2
    (`PrimitiveComponent.AddForceAtLocation` (`self.Box`) (* (* (`SceneComponent.GetUpVector` _thruster) (`self.ThrusterStrenght`)) (`KismetMathLibrary.FMin` (/ (`KismetMathLibrary.FClamp` (- 100.0 (`.Distance` (`GameplayStatics.BreakHitResult` _outhit))) 0.0 100.0) 100.0) 0.7)) (`SceneComponent.K2_GetComponentLocation` _thruster) "None")
    (`/Engine/EditorBlueprintResources/StandardMacros.IncrementInt` (`self.Thruster Hits`)
      (:`  `
        (return true)))
    (else
      (return false))))

(fn `GetGuns`
  (returns (NewParam :type "Array of /Game/HoverGame/Weapons/BP_HovercraftGun Object Reference"))
  (locals (Guns :type "Array of /Game/HoverGame/Weapons/BP_HovercraftGun Object Reference"))
  (`|ExecutionSequence`
    (:`then_0`
      (bind _asbp_hovercraft_gun (cast `/Game/HoverGame/Weapons/BP_HovercraftGun` (`ChildActorComponent.ChildActor` (`self.ChildActor1`))))
      (`KismetArrayLibrary.Array_Add` (`local.Guns`) _asbp_hovercraft_gun))
    (:`then_1`
      (bind _asbp_hovercraft_gun_2 (cast `/Game/HoverGame/Weapons/BP_HovercraftGun` (`ChildActorComponent.ChildActor` (`self.ChildActor`))))
      (`KismetArrayLibrary.Array_Add` (`local.Guns`) _asbp_hovercraft_gun_2))
    (:`then_2`
      (return (`local.Guns`)))))

(fn `LaunchMisileAt`
  (params (Target :type "Actor Object Reference"))
  (locals (NewLocalVar_0 :type "Transform Structure"))
  (bind (_returnvalue_location _returnvalue_rotation) (`KismetMathLibrary.BreakTransform` (`SceneComponent.K2_GetComponentToWorld` (`self.MissilePoint`))))
  (bind _returnvalue (`|SpawnActorFromClass` "/Game/HoverGame/Weapons/BP_TargetMissile.BP_TargetMissile_C" (`KismetMathLibrary.MakeTransform` _returnvalue_location _returnvalue_rotation) "Undefined" "OverrideRootScale" null null))
  (bind _projectilemovement (`/Game/HoverGame/Weapons/BP_TargetMissile.ProjectileMovement` _returnvalue))
  (set `MovementComponent.Velocity` (0.0 0.0 1000.0) _projectilemovement)
  (set `ProjectileMovementComponent.HomingTargetComponent` (`self.GetComponentByClass` Target "/Script/HoverGame.TargetComponent") _projectilemovement))

(fn `UpdateInput`
  (bind (_x _y) (`KismetMathLibrary.BreakRotIntoAxes` (`KismetMathLibrary.RLerp` (`self.K2_GetActorRotation`) (`self.GetControlRotation`) 0.5 true)))
  (`self.AddControllerYawInput` (`self.GetInputAxisValue`))
  (`self.AddControllerPitchInput` (`self.GetInputAxisValue`))
  (`self.AddMovementInput` (+ (* _x (`self.GetInputAxisValue`)) (* _y (`self.GetInputAxisValue`)))))

(fn `UpdateTargetting`
  (params (DeltaSeconds :type "Float (double-precision)"))
  (`TargetSelectionComponent.UpdateTargetting` (`self.TargetSelection`) (`SceneComponent.K2_GetComponentToWorld` (`self.Camera`)) DeltaSeconds (`self.SelectTargets`)))

(fn `UserConstructionScript`)