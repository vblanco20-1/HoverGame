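; BP_EnemyRobot is an AI enemy that wanders and fires its child-actor BP_RobotGun at the player.
; A looping timed trace finds random surface points around a wander origin, and the AIController moves there without pathfinding.
; When the player is within range, Tick aims and fires, recenters wandering on the player and sets a walk speed that is never reset.
; On death, it enables sphere physics, removes gun and target components, then destroys itself after a delay.
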(event `self.ReceiveBeginPlay`
  (bind _returnvalue (+ (* (`KismetMathLibrary.RandomUnitVector`) 10000.0) (`self.WanderOrigin`)))
  (bind _asbp_robot_gun (cast `/Game/HoverGame/Weapons/BP_RobotGun` (`ChildActorComponent.ChildActor` (`self.Gun`))))
  (set `self.RoboGun` _asbp_robot_gun)
  (set `self.WanderOrigin` (`self.K2_GetActorLocation`))
  ;[1 1 1] Random Walk
  (bind _outhit (`KismetSystemLibrary.LineTraceSingle` (+ _returnvalue (0.0 0.0 10000.0)) (+ _returnvalue (0.0 0.0 -10000.0)) "TraceTypeQuery1" :!label _label))
  (`AIController.MoveToLocation` (cast `AIController` (`self.GetController`) :!pure true) (`.Location` (`GameplayStatics.BreakHitResult` _outhit)) -1.0 true false false true null true)
  (`KismetSystemLibrary.Delay` 5.0)
  (goto _label))

(event `self.ReceiveTick`
  (params (DeltaSeconds :type "Float (single-precision)"))
  (bind _returnvalue (`GameplayStatics.GetPlayerPawn` 0))
  (bind _robogun (`self.RoboGun`))
  (bind _returnvalue_2 (`self.K2_GetActorLocation` _returnvalue))
  ;[1 1 1] Fire Logic
  (`/Engine/EditorBlueprintResources/StandardMacros.IsValid` (`self.RoboGun`)
    (:`Is Valid`
      (`/Engine/EditorBlueprintResources/StandardMacros.CompareFloat` (`self.GetDistanceTo` _returnvalue self) 10000.0
        (:`>`
          (set `/Game/HoverGame/Weapons/BP_RobotGun.Fire` false (`self.RoboGun`)))
        (:`<`
          (`/Game/HoverGame/Weapons/BP_RobotGun.SetTarget` _robogun _returnvalue_2)
          (set `/Game/HoverGame/Weapons/BP_RobotGun.Fire` true _robogun)
          (set `self.WanderOrigin` _returnvalue_2)
          (set `CharacterMovementComponent.MaxWalkSpeed` 2000.0 (`self.CharacterMovement`)))))))

(event `self.Damage.OnDeath`
  (params (Event :type "HoverDeathEvent Structure"))
  ;[1 1 1] Death Logic
  (`PrimitiveComponent.SetSimulatePhysics` (`self.Sphere`) true)
  (`ActorComponent.K2_DestroyComponent` (`self.Gun`))
  (`ActorComponent.K2_DestroyComponent` (`self.Target`))
  (`KismetSystemLibrary.Delay` 5.0)
  (`self.K2_DestroyActor`))

(fn `UserConstructionScript`)