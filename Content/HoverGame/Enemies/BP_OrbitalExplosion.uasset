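; BP_OrbitalExplosion is a delayed area strike in HoverGame's enemy set that homes toward a target location, then explodes.
; Tick moves the actor toward TargetLocation at Velocity while FollowTarget is set, stopping when close.
; BeginPlay runs a timed sequence that stops the following, pauses briefly to lock the impact point, then spawns a scaled explosion emitter, applies full radial damage and destroys the actor.
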(event `self.ReceiveBeginPlay`
  ;[1 1 1] Lifetime logic
  (`KismetSystemLibrary.Delay` 3.0)
  (set `self.FollowTarget` false)
  (`KismetSystemLibrary.Delay` 1.0)
  (bind _returnvalue (`GameplayStatics.SpawnEmitterAtLocation` "/Game/StarterContent/Particles/P_Explosion.P_Explosion" (`SceneComponent.K2_GetComponentLocation` (`self.DefaultSceneRoot`))))
  (`SceneComponent.SetWorldScale3D` _returnvalue (3.0 3.0 3.0))
  (`GameplayStatics.ApplyRadialDamage` 50.0 (+ (`SceneComponent.K2_GetComponentLocation` (`self.DefaultSceneRoot`)) (0.0 0.0 100.0)) 700.0 "/Script/Engine.DamageType" (`|MakeArray` self :!type "Actor Object Reference") self null true "ECC_Vehicle")
  (`self.K2_DestroyActor`))

(event `self.ReceiveTick`
  (params (DeltaSeconds :type "Float (single-precision)"))
  (bind _returnvalue (- (`self.TargetLocation`) (`SceneComponent.K2_GetComponentLocation` (`self.DefaultSceneRoot`))))
  ;[1 1 1] Tick: Move towards Target Location
  (if (and (`self.FollowTarget`) (> (`KismetMathLibrary.VSize` _returnvalue) 100.0))
    (`self.K2_AddActorWorldOffset` (* (`KismetMathLibrary.Normal` _returnvalue) (* DeltaSeconds (`self.Velocity`))))))

(fn `UserConstructionScript`)