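; Laser turret enemy that tracks the player pawn and fires a charged beam when the player is in range.
; A line trace starts the Ray timeline unless it hits Landscape or nothing, which stops it.
; Ray animates the beam material's width, freezes aiming, then fires a multi-sphere trace that damages actors with a DamageComponent.
; On death it stops the timeline, removes its Target component and hides the beam.
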(event `self.ReceiveBeginPlay`
  (bind _returnvalue (`PrimitiveComponent.CreateDynamicMaterialInstance` (`self.FXCylinder`) 0 null))
  (set `self.LaserMaterial` _returnvalue))

(event `self.ReceiveTick`
  (params (DeltaSeconds :type "Float (single-precision)"))
  (bind _returnvalue (`GameplayStatics.GetPlayerPawn` 0))
  (bind _firepoint (`self.FirePoint`))
  (bind _returnvalue_2 (`SceneComponent.K2_GetComponentLocation` _firepoint))
  (if (`DamageComponent.IsDead` (`self.Damage`))
    (`SceneComponent.SetVisibility` (`self.FXCylinder`) false false)
    (else
      (`|ExecutionSequence`
        (:`then_0`
          ;[1 1 1] Aiming
          (if (`self.AimAtPlayer`)
            (`self.LookAtPlayer`)))
        (:`then_1`
          ;[1 1 1] Check line of sight to player
          (if (< (`self.GetDistanceTo` _returnvalue) 10000.0)
            (bind _outhit (`KismetSystemLibrary.LineTraceSingle` (`SceneComponent.K2_GetComponentLocation` (`self.Scene`)) (`self.K2_GetActorLocation` _returnvalue) "TraceTypeQuery1"))
            (bind (_bblockinghit _binitialoverlap _time _distance _location _impactpoint _normal _impactnormal _physmat _hitactor) (`GameplayStatics.BreakHitResult` _outhit))
            (if _bblockinghit
              (cast `Landscape` _hitactor
                (:`then`
                  ;[1 1 1] Update Laser animation
                  (`|ExecutionSequence` :!label _label
                    (:`then_0`
                      (bind (_direction _lookatplayer _lasersize) (`Timeline|Ray` :!via `Stop` :!label _label_2)
                        (:`Update`
                          (`MaterialInstanceDynamic.SetScalarParameterValue` (`self.LaserMaterial`) "LaserWidth" (* (.x _lasersize) 100.0)))
                        (:`Finished`
                          (set `self.Shooting` false)
                          (set `self.AimAtPlayer` true)
                          (goto _label_3 :!via `Reset`))
                        (:`Freeze`
                          (set `self.AimAtPlayer` false))
                        (:`Fire`
                          ;[1 1 1] Perform Damage
                          (bind _outhits (`KismetSystemLibrary.SphereTraceMulti` _returnvalue_2 (+ _returnvalue_2 (* (`SceneComponent.GetForwardVector` _firepoint) 100000.0)) 50.0 "TraceTypeQuery1"))
                          (for _array_element _outhits
                            (bind _returnvalue_3 (`self.GetComponentByClass` (`.HitActor` (`GameplayStatics.BreakHitResult` _array_element)) "/Script/HoverGame.DamageComponent"))
                            (`/Engine/EditorBlueprintResources/StandardMacros.IsValid` _returnvalue_3
                              (:`Is Valid`
                                (`DamageComponent.ApplyDamage` :`self` _returnvalue_3 :`BaseDamage` 60.0 :`DamageCauser` self)))))))
                    (:`then_1`
                      (set `self.Shooting` false)
                      (`|ExecutionSequence`
                        (:`then_0`
                          (goto _label_3 :!via `Reset`))))))
                (:`CastFailed`
                  (set `self.Shooting` true)
                  (`/Engine/EditorBlueprintResources/StandardMacros.DoOnce` false :!label _label_3
                    (:`Completed`
                      (goto _label_2 :!via `PlayFromStart`)))))
              (else
                (goto _label)))))
        (:`then_2`
          ;[1 1 1] Laser Activation
          (`SceneComponent.SetVisibility` (`self.FXCylinder`) (`self.Shooting`) false))))))

(event `self.Damage.OnDeath`
  (params (Event :type "HoverDeathEvent Structure"))
  ;[1 1 1] Death Logic
  (`ActorComponent.K2_DestroyComponent` (`self.Target`))
  (goto _label_2 :!via `Stop`))

(fn `LookAtPlayer`
  (bind _scene (`self.Scene`))
  (`SceneComponent.K2_SetWorldRotation` _scene (`KismetMathLibrary.FindLookAtRotation` (`SceneComponent.K2_GetComponentLocation` _scene) (`self.K2_GetActorLocation` (`GameplayStatics.GetPlayerPawn` 0))) false false))

(fn `UserConstructionScript`)