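; BP_Bullet is a weapon projectile that deals damage and explodes on impact.
; When the projectile movement reports a bounce, it passes the hit to the target's DamageComponent if one exists, otherwise it uses standard Apply Damage.
; It then spawns an explosion emitter at the impact location and destroys itself, so the first bounce acts as the hit.
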(event `self.ProjectileMovement.OnProjectileBounce`
  (params (ImpactResult :type "HitResult Structure (by ref)") (ImpactVelocity :type "Vector Structure (by ref)"))
  (bind (_bblockinghit _binitialoverlap _time _distance _location _impactpoint _normal _impactnormal _physmat _hitactor) (`GameplayStatics.BreakHitResult` ImpactResult))
  (bind _returnvalue (`self.GetComponentByClass` _hitactor "/Script/HoverGame.DamageComponent"))
  (`|ExecutionSequence`
    (:`then_0`
      (`/Engine/EditorBlueprintResources/StandardMacros.IsValid` _returnvalue
        (:`Is Valid`
          (`DamageComponent.ApplyDamage` _returnvalue ImpactResult "/Script/Engine.DamageType" (`self.BaseDamage`) null self))
        (:`Is Not Valid`
          (`GameplayStatics.ApplyDamage` _hitactor (`self.BaseDamage`) null self "/Script/Engine.DamageType"))))
    (:`then_1`
      (`GameplayStatics.SpawnEmitterAtLocation` "/Game/StarterContent/Particles/P_Explosion.P_Explosion" _location)
      (`self.K2_DestroyActor`))))

(fn `UserConstructionScript`)