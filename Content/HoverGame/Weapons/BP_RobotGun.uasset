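; BP_RobotGun is a robot weapon actor that turns at a constant rate toward a target location supplied through SetTarget.
; While Fire is set, Tick runs a cooldown timer that spawns BP_RobotBullet at FirePoint at a fixed interval.
; A separate Shotgun function sprays BP_Bullets in a wide, flat random cone and kicks the attach parent's owner backward with a velocity impulse on its BoxComponent.
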(event `self.ReceiveTick`
  (params (DeltaSeconds :type "Float (single-precision)"))
  (`|ExecutionSequence`
    (:`then_0`
      (`self.K2_SetActorRotation` (`KismetMathLibrary.RInterpTo_Constant` (`self.K2_GetActorRotation`) (`KismetMathLibrary.FindLookAtRotation` (`self.K2_GetActorLocation`) (`self.TargetLocation`)) DeltaSeconds 60.0)))
    (:`then_1`
      (bind _output_get (set `self.ToNextShot` (- (`self.ToNextShot`) DeltaSeconds)))
      (if (`self.Fire`)
        (`/Engine/EditorBlueprintResources/StandardMacros.CompareFloat` _output_get
          (:`<`
            (set `self.ToNextShot` 0.2)
            (`|SpawnActorFromClass` "/Game/HoverGame/Weapons/BP_RobotBullet.BP_RobotBullet_C" (`KismetMathLibrary.MakeTransform` (.location (`SceneComponent.K2_GetComponentToWorld` (`self.FirePoint`))) (.rotation (`SceneComponent.K2_GetComponentToWorld` (`self.FirePoint`)))) "Undefined" "OverrideRootScale" null null)))))))

(fn `SetTarget`
  (params (TargetLocation :type "Vector Structure"))
  (set `self.TargetLocation` TargetLocation))

(fn `Shotgun`
  (for _ (range 9)
    (`|SpawnActorFromClass` "/Game/HoverGame/Weapons/BP_Bullet.BP_Bullet_C" (`KismetMathLibrary.MakeTransform` (.location (`SceneComponent.K2_GetComponentToWorld` (`self.FirePoint`))) (`KismetMathLibrary.MakeRotFromX` (`KismetMathLibrary.RandomUnitVectorInEllipticalConeInDegrees` (`KismetMathLibrary.GetForwardVector` (.rotation (`SceneComponent.K2_GetComponentToWorld` (`self.FirePoint`)))) 20.0 5.0))) "Undefined" "OverrideRootScale" null null))
  (`PrimitiveComponent.AddImpulse` (`self.GetComponentByClass` (`ActorComponent.GetOwner` (`SceneComponent.GetAttachParent` (`self.DefaultSceneRoot`))) "/Script/Engine.BoxComponent") (* (`SceneComponent.GetForwardVector` (`self.FirePoint`)) -1000.0) "None" true))

(fn `UserConstructionScript`)