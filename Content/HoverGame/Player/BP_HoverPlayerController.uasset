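; BP_HoverPlayerController is the HoverGame player controller that handles opening the pause menu and switching input modes.
; Backspace or Escape calls PauseGame, then creates a new WBP_PauseMenu widget and adds it to the viewport.
; OnPaused switches to UI-only input with a visible cursor, while OnUnpaused restores game-only input, unpauses the game and hides the cursor.
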(event `Key|BackSpace`
  (params (Key :type "Key Structure"))
  (:`Pressed`
    (`self.PauseGame` :!label _label)
    (bind _returnvalue (`|CreateWidget` "/Game/HoverGame/UI/WBP_PauseMenu.WBP_PauseMenu_C" self))
    (`UserWidget.AddToViewport` _returnvalue 0)))

(event `Key|Escape`
  (params (Key :type "Key Structure"))
  (:`Pressed`
    (goto _label)))

(event `self.OnPaused`
  (`WidgetBlueprintLibrary.SetInputMode_UIOnlyEx` self null "LockOnCapture")
  (set `self.bShowMouseCursor` true))

(event `self.OnUnpaused`
  (`WidgetBlueprintLibrary.SetInputMode_GameOnly` self)
  (`GameplayStatics.SetGamePaused` false)
  (set `self.bShowMouseCursor` false))

(fn `UserConstructionScript`)