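; BP_PointOfInterest is an actor that marks a point of interest with a widget showing a label and the player's distance to it.
; On BeginPlay and every Tick it casts its Widget component's user widget to WBP_POI and refreshes both texts.
; The label comes from the Text variable, and the distance is the horizontal distance to player pawn 0, converted to meters with one decimal.
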(event `self.ReceiveBeginPlay`
  (bind _aswbp_poi (cast `/Game/HoverGame/UI/WBP_POI` (`WidgetComponent.GetUserWidgetObject` (`self.Widget`)) :!label _label))
  (`TextBlock.SetText` (`/Game/HoverGame/UI/WBP_POI.DisplayText` _aswbp_poi) (`KismetTextLibrary.Conv_StringToText` (`self.Text`)))
  (`TextBlock.SetText` (`/Game/HoverGame/UI/WBP_POI.DistanceText` _aswbp_poi) (`|FormatText` "{dist}m" (`KismetTextLibrary.Conv_DoubleToText` (/ (`self.GetHorizontalDistanceTo` (`GameplayStatics.GetPlayerPawn` 0)) 100.0) "HalfToEven" false true 1 324 1 1))))

(event `self.ReceiveTick`
  (params (DeltaSeconds :type "Float (single-precision)"))
  (goto _label))

(fn `UserConstructionScript`)