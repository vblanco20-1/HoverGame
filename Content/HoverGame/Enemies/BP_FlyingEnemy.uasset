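; Flying enemy actor that wanders around its spawn point, or around the player once they have come within range of its periodic check.
; A five-second loop picks mostly horizontal random directions, which Tick smooths into an offset from that origin and moves toward with swept world offsets.
; A downward trace biases the direction to hold altitude above the floor.
; On death it simulates physics, removes its Target component and is destroyed after a delay.
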(event `CheckPlayer`
  (bind _returnvalue (`GameplayStatics.GetPlayerPawn` 0))
  (`/Engine/EditorBlueprintResources/StandardMacros.CompareFloat` (`self.GetDistanceTo` _returnvalue self) 20000.0
    (:`<`
      (set `self.TargetActor` _returnvalue))))

(event `self.ReceiveBeginPlay`
  (`KismetSystemLibrary.K2_SetTimerDelegate` (delegate `CheckPlayer`) 1.0 true)
  (set `self.StartLocation` (`self.K2_GetActorLocation`))
  (bind _output_get (set `self.DesiredMovement` (`KismetMathLibrary.RandomUnitVector`) :!label _label))
  (set `self.DesiredMovement` (`KismetMathLibrary.Normal` (* _output_get (1.0 1.0 0.1))))
  (`KismetSystemLibrary.Delay` 5.0)
  (goto _label))

(event `self.ReceiveTick`
  (params (DeltaSeconds :type "Float (single-precision)"))
  ;[1 1 1] MovementLogic
  (`self.CalcFloor`)
  (bind _output_get (set `self.CurrentMovement` (`KismetMathLibrary.VLerp` (`self.DesiredMovement`) (`self.CurrentMovement`) 0.9)))
  (bind _returnvalue (- (+ (* _output_get 1000.0) (`self.GetMovementOrigin`)) (`self.K2_GetActorLocation`)))
  (if (> (`KismetMathLibrary.VSize` _returnvalue) 100.0)
    (`self.K2_AddActorWorldOffset` (* (`KismetMathLibrary.Normal` _returnvalue) (* DeltaSeconds 500.0)) true)))

(event `self.Damage.OnDeath`
  (params (Event :type "HoverDeathEvent Structure"))
  ;[1 1 1] Death Logic
  (`PrimitiveComponent.SetSimulatePhysics` (`self.StaticMesh`) true)
  (`ActorComponent.K2_DestroyComponent` (`self.Target`))
  (`KismetSystemLibrary.Delay` 5.0)
  (`self.K2_DestroyActor`))

(fn `CalcFloor`
  (bind _returnvalue (`self.K2_GetActorLocation`))
  (bind (_outhit _returnvalue_2) (`KismetSystemLibrary.LineTraceSingle` _returnvalue (+ _returnvalue (0.0 0.0 -2000.0)) "TraceTypeQuery1"))
  (if _returnvalue_2
    (`/Engine/EditorBlueprintResources/StandardMacros.CompareFloat` (`.Distance` (`GameplayStatics.BreakHitResult` _outhit)) 1000.0
      (:`<`
        (set `self.DesiredMovement` (`KismetMathLibrary.Normal` (+ (`self.DesiredMovement`) (0.0 0.0 1.0))))))
    (else
      (set `self.DesiredMovement` (`KismetMathLibrary.Normal` (+ (`self.DesiredMovement`) (0.0 0.0 -1.0)))))))

(fn `GetMovementOrigin`
  (returns (NewParam :type "Vector Structure"))
  (`/Engine/EditorBlueprintResources/StandardMacros.IsValid` (`self.TargetActor`)
    (:`Is Valid`
      (return (`self.K2_GetActorLocation` (`self.TargetActor`))))
    (:`Is Not Valid`
      (return (`self.StartLocation`)))))

(fn `UserConstructionScript`)